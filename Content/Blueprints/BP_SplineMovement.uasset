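; Spline path actor that moves an array of referenced actors along its spline in a continuous loop, matching their position and rotation to the curve.
; The construction script pre-places each actor at its index times a spacing offset.
; At runtime a timeline, with play rate derived from a length setting, drives the shared distance, adds each actor's offset, wraps past the spline end and restarts when finished.
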(event Custom|PlayTime%20Line
  (bind _spline (Variables|Default|GetSpline))
  (bind _spline_2 (Variables|Default|GetSpline))
  (bind _returnvalue (Spline|GetSplineLength _spline))
  (bind _alpha (Timeline|Timeline PlayFromStart)
    (:Update
      (for (_array_element _array_index) (Variables|Default|GetActor)
        (bind _output_get (Variables|Default|SetDistance%20Along%20Spline (+ (Math|Float|Lerp 0.0 (Spline|GetSplineLength (Variables|Default|GetSpline)) _alpha) (* _array_index (Variables|Default|GetOffset%20Btween%20Actors)))))
        (if (> _output_get _returnvalue)
          (Variables|Default|SetDistance%20Along%20Spline (- (Variables|Default|GetDistance%20Along%20Spline) _returnvalue)))
        (Transformation|SetActorLocationAndRotation _array_element (Spline|GetLocationatDistanceAlongSpline _spline_2 (Variables|Default|GetDistance%20Along%20Spline) "World") (Spline|GetRotationatDistanceAlongSpline _spline_2 (Variables|Default|GetDistance%20Along%20Spline) "World"))))
    (:Finished
      (CallFunction|PlayTimeLine))))

(event EventBeginPlay
  (Components|Timeline|SetPlayRate (Variables|Default|GetTimeline) (/ 1.0 (Variables|Default|GetTimeLine%20Lenght)))
  (CallFunction|PlayTimeLine))

(fn ConstructionScript
  (bind _spline (Variables|Default|GetSpline))
  (for (_array_element _array_index) (Variables|Default|GetActor)
    (Transformation|SetActorLocationAndRotation _array_element (Spline|GetLocationatDistanceAlongSpline _spline (* _array_index (Variables|Default|GetOffset%20Btween%20Actors)) "World") (Spline|GetRotationatDistanceAlongSpline _spline (* _array_index (Variables|Default|GetOffset%20Btween%20Actors)) "World"))))