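; BP_EnemyProyectile is an enemy projectile that damages the player on contact.
; On BeginPlay it caches the first player state as PS_ShipState, unused in these graphs, then destroys itself after a five-second delay if that cast succeeds.
; Its Sphere overlap checks for the Player tag, prints the hit actor's name, applies fixed damage and destroys the projectile.
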(event OnComponentBeginOverlap(Sphere)
  (params (OverlappedComponent :type Primitive%20Component%20Object%20Reference) (OtherActor :type Actor%20Object%20Reference) (OtherComp :type Primitive%20Component%20Object%20Reference) (OtherBodyIndex :type Integer) (bFromSweep :type Boolean) (SweepResult :type Hit%20Result%20Structure%20%28by%20ref%29))
  (Utilities|IsValid OtherActor
    (:Is%20Valid
      (if (Actor|ActorHasTag OtherActor "Player")
        (Development|PrintString (Utilities|GetDisplayName OtherActor) true true "(R=0.000000,G=0.660000,B=1.000000,A=1.000000)" 2.0 "Hit")
        (Game|Damage|ApplyDamage OtherActor 2e+01 0 0)
        (Actor|DestroyActor)))))

(event EventBeginPlay
  (bind _asps_ship_state (Utilities|Casting|CastToPS_ShipState (Game|GetPlayerState 0)))
  (Variables|Default|SetAs%20PS%20Ship%20State _asps_ship_state)
  (Utilities|FlowControl|Delay 5.0)
  (Actor|DestroyActor))

(fn ConstructionScript)