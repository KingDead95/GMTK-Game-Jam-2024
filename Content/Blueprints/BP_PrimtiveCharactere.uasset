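; BP_PrimtiveCharactere is a player character moved sideways by a value read from its HUD widget.
; BeginPlay creates WB_HUD, adds it to the viewport and enables input.
; Every Tick feeds the widget's ValueNob into AddMovementInput along the control rotation's right vector.
; An unconnected branch holds an alternative that shifts the StaticMesh along X, reversing the offset past a threshold.
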(event EventBeginPlay
  (bind _returnvalue (UserInterface|CreateWidget "/Game/Blueprints/WB_HUD.WB_HUD_C"))
  (bind _output_get (Variables|Default|SetHUD _returnvalue))
  (UserInterface|Viewport|AddtoViewport _output_get 0)
  (Input|EnableInput self 0))

(event EventTick
  (params (DeltaSeconds :type Float%20%28single-precision%29))
  (bind _returnvalue (Pawn|GetControlRotation :!class /Script/Engine.Pawn))
  (Pawn|Input|AddMovementInput (Math|Vector|GetRightVector (Math|Rotator|MakeRotator (.roll _returnvalue) 0.0 (.yaw _returnvalue))) (Variables|/Game/Blueprints/WB_HUD.WB_HUD_C|GetValueNob (Variables|Default|GetHUD)) false))

(fn ConstructionScript)