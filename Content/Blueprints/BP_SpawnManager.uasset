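; Spawn manager that runs ship spawning across four zones of BP_SplineMovementPlayer actors.
; BeginPlay sorts those actors into zone arrays by actor tag and starts Zone 1, while separate events start Zones 2–4, each passing a larger vector to StarSpawn.
; Per-zone check functions report true when empty SpawnedShips counts reach the zone's size, using member counters that reset only on success, so counts accumulate between calls.
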(event Custom|SpawnZone2
  (Variables|Default|SetZone2%20Spaned true)
  (for _array_element (Variables|Default|GetZone2)
    (Default|StarSpawn _array_element "2.000000,2.000000,2.000000")))

(event Custom|SpawnZone3
  (for _array_element (Variables|Default|GetZone3)
    (Default|StarSpawn _array_element "3.000000,3.000000,3.000000"))
  (Variables|Default|SetZone3%20Spaned true))

(event Custom|SpawnZone4
  (for _array_element (Variables|Default|GetZone4)
    (Default|StarSpawn _array_element "4.000000,4.000000,4.000000"))
  (Variables|Default|SetZone4%20Spaned true))

(event EventBeginPlay
  (bind _outactors (Actor|GetAllActorsOfClass "/Game/Blueprints/BP_SplineMovementPlayer.BP_SplineMovementPlayer_C"))
  (for _array_element _outactors
    (if (Actor|ActorHasTag _array_element "Zone1")
      (Utilities|Array|Add (Variables|Default|GetZone1) _array_element)
      (elif (Actor|ActorHasTag _array_element "Zone2")
        (Utilities|Array|Add (Variables|Default|GetZone2) _array_element)
        (elif (Actor|ActorHasTag _array_element "Zone3")
          (Utilities|Array|Add (Variables|Default|GetZone3) _array_element)
          (elif (Actor|ActorHasTag _array_element "Zone4")
            (Utilities|Array|Add (Variables|Default|GetZone4) _array_element))))))
  (for _array_element_2 (Variables|Default|GetZone1)
    (Default|StarSpawn _array_element_2 "1.000000,1.000000,1.000000"))
  (Variables|Default|SetZone1%20Spaned true))

(fn ConstructionScript)

(fn ChecSwapns
  (if (Variables|Default|GetZone1%20Spaned)
    (for _array_element (Variables|Default|GetZone1)
      (if (Utilities|Array|IsEmpty (Variables|/Game/Blueprints/BP_SplineMovementPlayer.BP_SplineMovementPlayer_C|GetSpawned%20Ships _array_element))
        (bind _result (Math|Integer|IncrementInt (LocalVariables|GetIndex1)))))
    (if (>= (LocalVariables|GetIndex1) (Utilities|Array|Length (Variables|Default|GetZone1)))
      (LocalVariables|SetIndex1 0)
      (return true))))

(fn ChecSpanw2
  (if (Variables|Default|GetZone2%20Spaned)
    (for _array_element (Variables|Default|GetZone2)
      (if (Utilities|Array|IsEmpty (Variables|/Game/Blueprints/BP_SplineMovementPlayer.BP_SplineMovementPlayer_C|GetSpawned%20Ships _array_element))
        (bind _result (Math|Integer|IncrementInt (LocalVariables|GetIndex2)))))
    (if (>= (LocalVariables|GetIndex2) (Utilities|Array|Length (Variables|Default|GetZone2)))
      (LocalVariables|SetIndex2 0)
      (return true))))

(fn ChecSpawn3
  (if (Variables|Default|GetZone3%20Spaned)
    (for _array_element (Variables|Default|GetZone3)
      (if (Utilities|Array|IsEmpty (Variables|/Game/Blueprints/BP_SplineMovementPlayer.BP_SplineMovementPlayer_C|GetSpawned%20Ships _array_element))
        (bind _result (Math|Integer|IncrementInt (LocalVariables|GetInt4)))))
    (if (>= (LocalVariables|GetInt4) (Utilities|Array|Length (Variables|Default|GetZone3)))
      (LocalVariables|SetInt4 0)
      (return true))))

(fn ChecSapwns4
  (if (Variables|Default|GetZone4%20Spaned)
    (for _array_element (Variables|Default|GetZone4)
      (if (Utilities|Array|IsEmpty (Variables|/Game/Blueprints/BP_SplineMovementPlayer.BP_SplineMovementPlayer_C|GetSpawned%20Ships _array_element))
        (bind _result (Math|Integer|IncrementInt (LocalVariables|GetIndex4)))))
    (if (>= (LocalVariables|GetIndex4) (Utilities|Array|Length (Variables|Default|GetZone4)))
      (LocalVariables|SetIndex4 0)
      (return true))))