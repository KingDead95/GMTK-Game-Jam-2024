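; BP_Chamera is a camera actor that also drives zone progression and the win state.
; BeginPlay caches the spawn manager, player ship and blocking volume; Tick then polls zone flags and the ship core's world scale.
; Each zone cleared or scale threshold reached fires a DoOnce that lengthens the spring arm, enlarges the blocking volume and spawns the next zone.
; Completing Zone4 pauses the game and shows the WB_Won screen, with no DoOnce guard.
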(event EventBeginPlay
  (bind _returnvalue (Actor|GetActorOfClass "/Game/Blueprints/BP_SpawnManager.BP_SpawnManager_C"))
  (Variables|Default|SetSpawner _returnvalue)
  (bind _returnvalue_2 (Actor|GetActorOfClass "/Game/Characters/Ship/BP_PlayerShip.BP_PlayerShip_C"))
  (Variables|Default|SetBP_Player _returnvalue_2)
  (bind _returnvalue_3 (Actor|GetActorOfClass "/Script/Engine.BlockingVolume"))
  (bind _output_get (Variables|Default|SetBlockVolume _returnvalue_3))
  (Transformation|SetActorScale3D _output_get "20.000000,11.000000,2.000000"))

(event EventTick
  (params (DeltaSeconds :type Float%20%28single-precision%29))
  (bind _returnvalue (Game|GetPlayerController 0))
  (bind (_zone1 _zone2 _zone3 _zone4) (Default|ChecSwapns (Variables|Default|GetSpawner)))
  (Utilities|FlowControl|Sequence
    (:then_0
      (if (or _zone1 (>= (.x (Transformation|GetWorldScale (Variables|/Game/Characters/Ship/BP_PlayerShip.BP_PlayerShip_C|GetStarSparrow_Core (Variables|Default|GetBP_Player)))) 0.85))
        (Utilities|FlowControl|DoOnce false
          (:Completed
            (Variables|/Script/Engine.SpringArmComponent|SetTargetArmLength (Variables|Default|GetSpringArm) 5e+03)
            (Transformation|SetActorScale3D (Variables|Default|GetBlockVolume) "60.000000,21.500000,2.000000")
            (Default|SpawnZone2 (Variables|Default|GetSpawner))))))
    (:then_1
      (if (or _zone2 (>= (.x (Transformation|GetWorldScale (Variables|/Game/Characters/Ship/BP_PlayerShip.BP_PlayerShip_C|GetStarSparrow_Core (Variables|Default|GetBP_Player)))) 1.7))
        (Utilities|FlowControl|DoOnce false
          (:Completed
            (Variables|/Script/Engine.SpringArmComponent|SetTargetArmLength (Variables|Default|GetSpringArm) 1e+04)
            (Transformation|SetActorScale3D (Variables|Default|GetBlockVolume) "100.000000,45.500000,2.000000")
            (Default|SpawnZone3 (Variables|Default|GetSpawner))))))
    (:then_2
      (if (or _zone3 (>= (.x (Transformation|GetWorldScale (Variables|/Game/Characters/Ship/BP_PlayerShip.BP_PlayerShip_C|GetStarSparrow_Core (Variables|Default|GetBP_Player)))) 2.4))
        (Utilities|FlowControl|DoOnce false
          (:Completed
            (Variables|/Script/Engine.SpringArmComponent|SetTargetArmLength (Variables|Default|GetSpringArm) 2e+04)
            (Transformation|SetActorScale3D (Variables|Default|GetBlockVolume) "190.000000,95.000000,2.000000")
            (Default|SpawnZone4 (Variables|Default|GetSpawner))))))
    (:then_3
      (if _zone4
        (Game|SetGamePaused true)
        (bind _returnvalue_2 (UserInterface|CreateWidget "/Game/Blueprints/UI/menu/WB_Won.WB_Won_C" _returnvalue))
        (Input|SetInputModeUIOnly _returnvalue _returnvalue_2 "DoNotLock" false)
        (Variables|/Script/Engine.PlayerController|SetbShowMouseCursor _returnvalue true)
        (UserInterface|Viewport|AddtoViewport _returnvalue_2 0)))))

(fn ConstructionScript)