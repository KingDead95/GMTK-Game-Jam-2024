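; BP_BattleShip_Cyan is an enemy battleship that turns to face the player ship and fires projectile volleys at it.
; Tick interpolates its yaw toward BP_PlayerShip and is disabled when none is found.
; After a short delay, a self-re-entering Gate loop spawns BP_EnemyProyectile from four weapon sockets, paced by FireRate, until StopFiring closes it.
; Damage drains Life, a hit at zero or below destroys it, and destruction grants the player EXP.
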(event Custom|StarFiring
  (bind _defaultsceneroot (Variables|Default|GetDefaultSceneRoot))
  (bind _returnvalue (Transformation|GetWorldRotation _defaultsceneroot))
  (Utilities|FlowControl|Sequence
    (:then_0
      (goto _label Open))
    (:then_1
      (Utilities|FlowControl|Gate true :!label _label
        (:Exit
          (Utilities|FlowControl|Sequence
            (:then_0
              (Game|SpawnActorfromClass "/Game/Blueprints/BP_EnemyProyectile.BP_EnemyProyectile_C" (Math|Transform|MakeTransform (Transformation|GetSocketLocation (Variables|Default|GetStarSparrow_Weapon) "Fire") (Math|Rotator|MakeRotator (.roll _returnvalue) (.pitch _returnvalue) (- (.yaw _returnvalue) 2.7e+02)) "1.000000,1.000000,1.000000") "Undefined" "MultiplyWithRoot" 0 (Variables|Default|GetBullet%20Material) 0)
              (Game|SpawnActorfromClass "/Game/Blueprints/BP_EnemyProyectile.BP_EnemyProyectile_C" (Math|Transform|MakeTransform (Transformation|GetSocketLocation (Variables|Default|GetStarSparrow_Weapon3) "Fire") (Math|Rotator|MakeRotator 0.0 0.0 (- (.yaw (Transformation|GetWorldRotation (Variables|Default|GetDefaultSceneRoot))) 2.7e+02)) "1.000000,1.000000,1.000000") "Undefined" "MultiplyWithRoot" 0 (Variables|Default|GetBullet%20Material) 0)
              (Game|SpawnActorfromClass "/Game/Blueprints/BP_EnemyProyectile.BP_EnemyProyectile_C" (Math|Transform|MakeTransform (Transformation|GetSocketLocation (Variables|Default|GetStarSparrow_Weapon4) "Fire") (Math|Rotator|MakeRotator 0.0 0.0 (- (.yaw (Transformation|GetWorldRotation (Variables|Default|GetDefaultSceneRoot))) 2.7e+02)) "1.000000,1.000000,1.000000") "Undefined" "MultiplyWithRoot" 0 (Variables|Default|GetBullet%20Material) 0)
              (Game|SpawnActorfromClass "/Game/Blueprints/BP_EnemyProyectile.BP_EnemyProyectile_C" (Math|Transform|MakeTransform (Transformation|GetSocketLocation (Variables|Default|GetStarSparrow_Weapon5) "Fire") (Math|Rotator|MakeRotator 0.0 0.0 (- (.yaw (Transformation|GetWorldRotation (Variables|Default|GetDefaultSceneRoot))) 2.7e+02)) "1.000000,1.000000,1.000000") "Undefined" "MultiplyWithRoot" 0 (Variables|Default|GetBullet%20Material) 0))
            (:then_1
              (Utilities|FlowControl|Delay (* 1.0 (Variables|Default|GetFireRate)))
              (goto _label))))))))

(event Custom|StopFiring
  (bind _defaultsceneroot (Variables|Default|GetDefaultSceneRoot))
  (bind _returnvalue (Transformation|GetWorldRotation _defaultsceneroot))
  (Utilities|FlowControl|Gate true) ; enters at Close
)

(event EventBeginPlay
  (bind _returnvalue (Actor|GetActorOfClass "/Game/Characters/Ship/BP_PlayerShip.BP_PlayerShip_C"))
  (Variables|Default|SetPlayerShip _returnvalue)
  (Utilities|IsValid _returnvalue
    (:Is%20Valid
      (Actor|Tick|SetActorTickEnabled true)
      (Utilities|FlowControl|Delay 1.0)
      (CallFunction|StarFiring))
    (:Is%20Not%20Valid
      (Actor|Tick|SetActorTickEnabled false))))

(event EventTick
  (params (DeltaSeconds :type Float%20%28single-precision%29))
  (bind _playership (Variables|Default|GetPlayerShip))
  (bind _defaultsceneroot (Variables|Default|GetDefaultSceneRoot))
  (bind _returnvalue (Transformation|GetWorldLocation _defaultsceneroot))
  (bind _box (Variables|/Game/Characters/Ship/BP_PlayerShip.BP_PlayerShip_C|GetBox _playership))
  (bind _returnvalue_2 (Transformation|GetWorldLocation _box))
  (bind _returnvalue_3 (Math|Rotator|FindLookatRotation _returnvalue _returnvalue_2))
  (Transformation|SetWorldRotation (Variables|Default|GetDefaultSceneRoot) (Math|Rotator|MakeRotator 0.0 0.0 (.yaw (Math|Interpolation|RInterpTo (Transformation|GetWorldRotation (Variables|Default|GetDefaultSceneRoot)) (Math|Rotator|MakeRotator (.roll _returnvalue_3) (.pitch _returnvalue_3) (+ (.yaw _returnvalue_3) 2.7e+02)) DeltaSeconds 0.0))) false false))

(event EventDestroyed
  (Default|GainEXP (Variables|/Game/Characters/Ship/BP_PlayerShip.BP_PlayerShip_C|GetPS%20Ship%20State (Variables|Default|GetPlayerShip)) 5.0))

(event Game|Damage|EventAnyDamage
  (params (Damage :type Float%20%28single-precision%29) (DamageType :type Damage%20Type%20Object%20Reference) (InstigatedBy :type Controller%20Object%20Reference) (DamageCauser :type Actor%20Object%20Reference))
  (if (> (Variables|Default|GetLife) 0.0)
    (Variables|Default|SetLife (- (Variables|Default|GetLife) Damage))
    (else
      (Actor|DestroyActor))))

(fn ConstructionScript)