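; Spline path actor that spawns a group of random ships from a class list and moves them along its spline.
; StarSpawn spawns them at the first spline point, waits briefly, then runs a rate-scaled Timeline forward or in reverse.
; Timeline updates set location only, spacing ships by index offset and wrapping past the spline's end.
; Tick prunes invalid ships; the player ship reference is cached but unused here.
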(event Custom|PlayTime%20Line
  (bind _spline (Variables|Default|GetSpline))
  (bind _returnvalue (Spline|GetSplineLength _spline))
  (bind _alpha (Timeline|Timeline PlayFromStart)
    (:Update
      (for (_array_element _array_index) (Variables|Default|GetSpawned%20Ships)
        (Utilities|IsValid _array_element
          (:Is%20Valid
            (bind _output_get (Variables|Default|SetDistance%20Along%20Spline (+ (Math|Float|Lerp 0.0 (Spline|GetSplineLength (Variables|Default|GetSpline)) _alpha) (* _array_index (Variables|Default|GetOffset%20Btween%20Actors)))))
            (if (> _output_get _returnvalue)
              (Variables|Default|SetDistance%20Along%20Spline (- (Variables|Default|GetDistance%20Along%20Spline) _returnvalue)))
            (Transformation|SetActorLocation _array_element (Spline|GetLocationatDistanceAlongSpline (Variables|Default|GetSpline) (Variables|Default|GetDistance%20Along%20Spline) "World") false false)))))))

(event Custom|PlayReverse
  (bind _spline (Variables|Default|GetSpline))
  (bind _returnvalue (Spline|GetSplineLength _spline))
  (bind _alpha (Timeline|Timeline ReverseFromEnd)
    (:Update
      (for (_array_element _array_index) (Variables|Default|GetSpawned%20Ships)
        (Utilities|IsValid _array_element
          (:Is%20Valid
            (bind _output_get (Variables|Default|SetDistance%20Along%20Spline (+ (Math|Float|Lerp 0.0 (Spline|GetSplineLength (Variables|Default|GetSpline)) _alpha) (* _array_index (Variables|Default|GetOffset%20Btween%20Actors)))))
            (if (> _output_get _returnvalue)
              (Variables|Default|SetDistance%20Along%20Spline (- (Variables|Default|GetDistance%20Along%20Spline) _returnvalue)))
            (Transformation|SetActorLocation _array_element (Spline|GetLocationatDistanceAlongSpline (Variables|Default|GetSpline) (Variables|Default|GetDistance%20Along%20Spline) "World") false false)))))))

(event Custom|StarSpawn
  (params (Spawn%20Transform%20Scale :type Vector))
  (CallFunction|SpawnShips (Variables|Default|GetShip%20Numbers) Spawn%20Transform%20Scale)
  (Utilities|FlowControl|Delay 1.0)
  (Components|Timeline|SetPlayRate (Variables|Default|GetTimeline) (/ 1.0 (Variables|Default|GetTimeLine%20Lenght)))
  (if (Variables|Default|GetPlayReverse?)
    (CallFunction|PlayReverse)
    (else
      (CallFunction|PlayTimeLine))))

(event EventBeginPlay
  (bind _returnvalue (Actor|GetActorOfClass "/Game/Characters/Ship/BP_PlayerShip.BP_PlayerShip_C"))
  (Variables|Default|SetPlayer _returnvalue))

(event EventTick
  (params (DeltaSeconds :type Float%20%28single-precision%29))
  (bind _spawned_ships (Variables|Default|GetSpawned%20Ships))
  (for _array_element _spawned_ships
    (Utilities|IsValid _array_element
      (:Is%20Not%20Valid
        (Utilities|Array|RemoveItem _spawned_ships _array_element)))))

(fn ConstructionScript)

(fn SpawnShips
  (params (LastIndex :type Integer) (Spawn%20Transform%20Scale :type Vector))
  (bind _classactor (Variables|Default|GetClassActor))
  (bind _classactor_2 (Variables|Default|GetClassActor))
  (bind _returnvalue (Utilities|Array|Length _classactor_2))
  (bind _returnvalue_2 (Math|Random|RandomIntegerinRange 0 _returnvalue))
  (for _index (range 0 LastIndex)
    (if (Utilities|Array|IsValidIndex _classactor _returnvalue_2)
      (bind _returnvalue_3 (Game|SpawnActorfromClass (Utilities|Array|Get(acopy) _classactor _returnvalue_2) (Math|Transform|MakeTransform (Spline|GetLocationatSplinePoint (Variables|Default|GetSpline) 0 "World") "0, 0, 0" Spawn%20Transform%20Scale) "AdjustIfPossibleButAlwaysSpawn" "MultiplyWithRoot" 0 0))
      (Utilities|Array|Add (Variables|Default|GetSpawned%20Ships) _returnvalue_3)
      (else
        (bind _returnvalue_4 (Game|SpawnActorfromClass (Utilities|Array|Get(acopy) (Variables|Default|GetClassActor)) (Math|Transform|MakeTransform (Spline|GetLocationatSplinePoint (Variables|Default|GetSpline) 0 "World") "0, 0, 0" Spawn%20Transform%20Scale) "AdjustIfPossibleButAlwaysSpawn" "MultiplyWithRoot" 0 0))
        (Utilities|Array|Add (Variables|Default|GetSpawned%20Ships) _returnvalue_4))))
  (return))