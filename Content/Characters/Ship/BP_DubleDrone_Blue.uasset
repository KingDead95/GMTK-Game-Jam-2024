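; Blue double drone actor that turns to face the player ship and grants experience when destroyed.
; On BeginPlay it caches the ship state and player ship, ticking only if the ship exists.
; Tick applies RInterpTo toward the ship's box with an offset, changing only yaw.
; Damage lowers Life; a hit arriving once Life is depleted awards EXP and destroys the drone after a short delay.
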(event EventBeginPlay
  (bind _returnvalue (Actor|GetActorOfClass "/Game/Blueprints/PS_ShipState.PS_ShipState_C"))
  (Variables|Default|SetPS _returnvalue)
  (bind _returnvalue_2 (Actor|GetActorOfClass "/Game/Characters/Ship/BP_PlayerShip.BP_PlayerShip_C"))
  (Variables|Default|SetPlayerShip _returnvalue_2)
  (Utilities|IsValid _returnvalue_2
    (:Is%20Valid
      (Actor|Tick|SetActorTickEnabled true))
    (:Is%20Not%20Valid
      (Actor|Tick|SetActorTickEnabled false))))

(event EventTick
  (params (DeltaSeconds :type Float%20%28single-precision%29))
  (bind _playership (Variables|Default|GetPlayerShip))
  (bind _defaultsceneroot (Variables|Default|GetDefaultSceneRoot))
  (bind _returnvalue (Transformation|GetWorldLocation _defaultsceneroot))
  (bind _box (Variables|/Game/Characters/Ship/BP_PlayerShip.BP_PlayerShip_C|GetBox _playership))
  (bind _returnvalue_2 (Transformation|GetWorldLocation _box))
  (bind _returnvalue_3 (Math|Rotator|FindLookatRotation _returnvalue _returnvalue_2))
  (Transformation|SetWorldRotation (Variables|Default|GetDefaultSceneRoot) (Math|Rotator|MakeRotator 0.0 0.0 (.yaw (Math|Interpolation|RInterpTo (Transformation|GetWorldRotation (Variables|Default|GetDefaultSceneRoot)) (Math|Rotator|MakeRotator (.roll _returnvalue_3) (.pitch _returnvalue_3) (+ (.yaw _returnvalue_3) 2.7e+02)) DeltaSeconds 0.0))) false false))

(event Game|Damage|EventAnyDamage
  (params (Damage :type Float%20%28single-precision%29) (DamageType :type Damage%20Type%20Object%20Reference) (InstigatedBy :type Controller%20Object%20Reference) (DamageCauser :type Actor%20Object%20Reference))
  (if (> (Variables|Default|GetLife) 0.0)
    (Variables|Default|SetLife (- (Variables|Default|GetLife) Damage))
    (else
      (Default|GainEXP (Variables|Default|GetPS) 2e+01)
      (Utilities|FlowControl|Delay 0.4)
      (Actor|DestroyActor))))

(fn ConstructionScript)